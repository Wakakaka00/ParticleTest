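; Anim notify state that lunges MyCharacter toward its close enemy during an animation, falling back to cached pre-attack direction or actor forward.
; Begin caches player position and physics flag, then always calls LaunchCharacter.
; Unless physics mode or reached flag is set, Tick also lerps location with sweep toward a point Units from that position.
; Two downward traces supply the slope angle that tilts movement; End zeroes velocity and clears the reached flag.
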(fn ReceivedNotifyTick
  (params (MeshComp :type Skeletal%20Mesh%20Component%20Object%20Reference) (Animation :type Anim%20Sequence%20Base%20Object%20Reference) (FrameDeltaTime :type Float%20%28single-precision%29))
  (bind _returnvalue (Components|GetOwner MeshComp))
  (bind _units (Variables|Default|GetUnits))
  (bind _speed (Variables|Default|GetSpeed))
  (bind _returnvalue_2 (Transformation|GetActorLocation _returnvalue))
  (bind _returnvalue_3 (* FrameDeltaTime _speed))
  (bind _asmy_character (Utilities|Casting|CastToMyCharacter _returnvalue))
  (if (not (Variables|/Game/Blueprints/MyTPSCharacter/MyCharacter.MyCharacter_C|GetMoveToward-BePhysics _asmy_character))
    (if (not (Variables|/Game/Blueprints/MyTPSCharacter/MyCharacter.MyCharacter_C|GetMoveToward-ReachAlready? _asmy_character))
      (bind (_angletoallign _angleitself) (|Ground (Game|GetPlayerCharacter _asmy_character) _asmy_character))
      (LocalVariables|SetRotatedForwardVectorSlope (Math|Vector|RotateVectorAroundAxis (Transformation|GetActorForwardVector _asmy_character) _angleitself (Transformation|GetActorRightVector _asmy_character)))
      (LocalVariables|SetRotatedCacheRotationSlope (Math|Vector|RotateVectorAroundAxis (Variables|/Game/Blueprints/MyTPSCharacter/MyCharacter.MyCharacter_C|GetCachedRotationBeforeAttack _asmy_character) _angleitself (Transformation|GetActorRightVector _asmy_character)))
      (Utilities|IsValid (Variables|/Game/Blueprints/MyTPSCharacter/MyCharacter.MyCharacter_C|GetTemperoryCloseEnemy _asmy_character)
        (:Is%20Valid
          (Transformation|SetActorLocation _asmy_character (Math|Vector|Lerp(Vector) _returnvalue_2 (Math|Vector|MakeVector (.x (+ (* (Math|Vector|RotateVector (Math|Vector|GetUnitDirection(Vector) (Variables|/Game/Blueprints/MyTPSCharacter/MyCharacter.MyCharacter_C|GetMoveToward-CashePlayerPositionBeforeMoving _asmy_character) (Transformation|GetActorLocation (Variables|/Game/Blueprints/MyTPSCharacter/MyCharacter.MyCharacter_C|GetTemperoryCloseEnemy _asmy_character))) _angletoallign) _units) (Variables|/Game/Blueprints/MyTPSCharacter/MyCharacter.MyCharacter_C|GetMoveToward-CashePlayerPositionBeforeMoving _asmy_character))) (.y (+ (* (Math|Vector|RotateVector (Math|Vector|GetUnitDirection(Vector) (Variables|/Game/Blueprints/MyTPSCharacter/MyCharacter.MyCharacter_C|GetMoveToward-CashePlayerPositionBeforeMoving _asmy_character) (Transformation|GetActorLocation (Variables|/Game/Blueprints/MyTPSCharacter/MyCharacter.MyCharacter_C|GetTemperoryCloseEnemy _asmy_character))) _angletoallign) _units) (Variables|/Game/Blueprints/MyTPSCharacter/MyCharacter.MyCharacter_C|GetMoveToward-CashePlayerPositionBeforeMoving _asmy_character))) (.z (Transformation|GetActorLocation _returnvalue))) _returnvalue_3) true false))
        (:Is%20Not%20Valid
          (if (> (Math|Vector|VectorLength (Variables|/Game/Blueprints/MyTPSCharacter/MyCharacter.MyCharacter_C|GetCachedRotationBeforeAttack _asmy_character)) 0.0)
            (Transformation|SetActorLocation _asmy_character (Math|Vector|Lerp(Vector) _returnvalue_2 (Math|Vector|MakeVector (.x (+ (Variables|/Game/Blueprints/MyTPSCharacter/MyCharacter.MyCharacter_C|GetMoveToward-CashePlayerPositionBeforeMoving _asmy_character) (* (LocalVariables|GetRotatedCacheRotationSlope) _units))) (.y (+ (Variables|/Game/Blueprints/MyTPSCharacter/MyCharacter.MyCharacter_C|GetMoveToward-CashePlayerPositionBeforeMoving _asmy_character) (* (LocalVariables|GetRotatedCacheRotationSlope) _units))) (.z (+ (Variables|/Game/Blueprints/MyTPSCharacter/MyCharacter.MyCharacter_C|GetMoveToward-CashePlayerPositionBeforeMoving _asmy_character) (* (LocalVariables|GetRotatedCacheRotationSlope) _units)))) _returnvalue_3) true false)
            (else
              (Transformation|SetActorLocation _asmy_character (Math|Vector|Lerp(Vector) _returnvalue_2 (Math|Vector|MakeVector (.x (+ (Variables|/Game/Blueprints/MyTPSCharacter/MyCharacter.MyCharacter_C|GetMoveToward-CashePlayerPositionBeforeMoving _asmy_character) (* (LocalVariables|GetRotatedForwardVectorSlope) _units))) (.y (+ (Variables|/Game/Blueprints/MyTPSCharacter/MyCharacter.MyCharacter_C|GetMoveToward-CashePlayerPositionBeforeMoving _asmy_character) (* (LocalVariables|GetRotatedForwardVectorSlope) _units))) (.z (+ (Variables|/Game/Blueprints/MyTPSCharacter/MyCharacter.MyCharacter_C|GetMoveToward-CashePlayerPositionBeforeMoving _asmy_character) (* (LocalVariables|GetRotatedForwardVectorSlope) _units)))) _returnvalue_3) true false)))
          (Rendering|Debug|DrawDebugArrow _asmy_character (Variables|/Game/Blueprints/MyTPSCharacter/MyCharacter.MyCharacter_C|GetMoveToward-CashePlayerPositionBeforeMoving _asmy_character) (+ (* (Math|Vector|RotateVectorAroundAxis (Variables|/Game/Blueprints/MyTPSCharacter/MyCharacter.MyCharacter_C|GetCachedRotationBeforeAttack _asmy_character) _angleitself (Transformation|GetActorRightVector _asmy_character)) 1e+02) (Variables|/Game/Blueprints/MyTPSCharacter/MyCharacter.MyCharacter_C|GetMoveToward-CashePlayerPositionBeforeMoving _asmy_character)) 4.0 "(R=1.000000,G=0.000000,B=0.055564,A=1.000000)" 2.0 2.0)
          (return false))))))

(fn ReceivedNotifyBegin
  (params (MeshComp :type Skeletal%20Mesh%20Component%20Object%20Reference) (Animation :type Anim%20Sequence%20Base%20Object%20Reference) (TotalDuration :type Float%20%28single-precision%29))
  (bind _returnvalue (Components|GetOwner MeshComp))
  (bind _asmy_character (Utilities|Casting|CastToMyCharacter (Game|Player|GetPlayerPawn MeshComp)))
  (Variables|/Game/Blueprints/MyTPSCharacter/MyCharacter.MyCharacter_C|SetMoveToward-CashePlayerPositionBeforeMoving _asmy_character (Transformation|GetActorLocation _asmy_character))
  (Variables|/Game/Blueprints/MyTPSCharacter/MyCharacter.MyCharacter_C|SetMoveToward-BePhysics _asmy_character (Variables|Default|GetbePhysicMove?))
  (if true
    (bind _asmy_character_2 (Utilities|Casting|CastToMyCharacter _returnvalue))
    (bind _angle (|Ground2 _asmy_character_2 _asmy_character_2))
    (LocalVariables|SetRotatedForwardVectorSlope (Math|Vector|RotateVectorAroundAxis (Transformation|GetActorForwardVector _asmy_character_2) _angle (Transformation|GetActorRightVector _asmy_character_2)))
    (LocalVariables|SetRotatedCacheRotationSlope (Math|Vector|RotateVectorAroundAxis (Variables|/Game/Blueprints/MyTPSCharacter/MyCharacter.MyCharacter_C|GetCachedRotationBeforeAttack _asmy_character_2) _angle (Transformation|GetActorRightVector _asmy_character_2)))
    (Utilities|IsValid (Variables|/Game/Blueprints/MyTPSCharacter/MyCharacter.MyCharacter_C|GetTemperoryCloseEnemy _asmy_character_2)
      (:Is%20Valid
        (Character|LaunchCharacter _asmy_character_2 (* (Math|Vector|RotateVectorAroundAxis (Math|Vector|MakeVector (.x (Math|Vector|GetUnitDirection(Vector) (Transformation|GetActorLocation _returnvalue) (Transformation|GetActorLocation (Variables|/Game/Blueprints/MyTPSCharacter/MyCharacter.MyCharacter_C|GetTemperoryCloseEnemy _asmy_character_2)))) (.y (Math|Vector|GetUnitDirection(Vector) (Transformation|GetActorLocation _returnvalue) (Transformation|GetActorLocation (Variables|/Game/Blueprints/MyTPSCharacter/MyCharacter.MyCharacter_C|GetTemperoryCloseEnemy _asmy_character_2)))) 0.0) _angle (Transformation|GetActorRightVector _asmy_character_2)) (Variables|Default|GetLaunchVelocityForPhysics)) true true))
      (:Is%20Not%20Valid
        (if (> (Math|Vector|VectorLength (Variables|/Game/Blueprints/MyTPSCharacter/MyCharacter.MyCharacter_C|GetCachedRotationBeforeAttack _asmy_character_2)) 0.0)
          (Character|LaunchCharacter _asmy_character_2 (* (LocalVariables|GetRotatedCacheRotationSlope) (Variables|Default|GetLaunchVelocityForPhysics)) true true)
          (else
            (Character|LaunchCharacter _asmy_character_2 (* (LocalVariables|GetRotatedForwardVectorSlope) (Variables|Default|GetLaunchVelocityForPhysics)) true true)))))
    (return true)))

(fn ReceivedNotifyEnd
  (params (MeshComp :type Skeletal%20Mesh%20Component%20Object%20Reference) (Animation :type Anim%20Sequence%20Base%20Object%20Reference))
  (bind _asmy_character (Utilities|Casting|CastToMyCharacter (Components|GetOwner MeshComp)))
  (Variables|/Script/Engine.MovementComponent|SetVelocity (Variables|/Script/Engine.Character|GetCharacterMovement _asmy_character) "0, 0, 0")
  (Variables|/Game/Blueprints/MyTPSCharacter/MyCharacter.MyCharacter_C|SetMoveToward-ReachAlready? _asmy_character false)
  (return false))