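; Anim notify state that opens a melee hit window during the player's sword attack animations.
; Each tick sphere-traces pawns between the sword sockets, filtering for components tagged DamageBody.
; It flags and records one new Enemy per tick, then calls MyCharacter's Damager with the attack type and a brief hit pause.
; On end, it calls the character's list cleanup unless the animation is paused, and re-enables hit pause.
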(fn ReceivedNotifyBegin
  (params (MeshComp :type Skeletal%20Mesh%20Component%20Object%20Reference) (Animation :type Anim%20Sequence%20Base%20Object%20Reference) (TotalDuration :type Float%20%28single-precision%29)))

(fn ReceivedNotifyTick
  (params (MeshComp :type Skeletal%20Mesh%20Component%20Object%20Reference) (Animation :type Anim%20Sequence%20Base%20Object%20Reference) (FrameDeltaTime :type Float%20%28single-precision%29))
  (Utilities|Casting|CastToMyCharacter (Game|GetPlayerCharacter MeshComp))
  (bind _outhits (Collision|MultiSphereTraceForObjects MeshComp (Transformation|GetSocketLocation MeshComp "FX_Sword_Bottom") (Transformation|GetSocketLocation MeshComp "FX_Sword_Top") 35.0 (Utilities|Array|MakeArray "ObjectTypeQuery3") false (Utilities|Array|MakeArray (Components|GetOwner MeshComp)) "None" true "(R=1.000000,G=0.000000,B=0.000000,A=1.000000)" "(R=0.000000,G=1.000000,B=0.000000,A=1.000000)" 0.1))
  (for _array_element _outhits
    (Utilities|IsValid (.hitcomponent _array_element)
      (:Is%20Valid
        (if (Components|ComponentHasTag (.hitcomponent _array_element) "DamageBody")
          (bind _asenemy (Utilities|Casting|CastToEnemy (Components|GetOwner (.hitcomponent _array_element))))
          (bind _returnvalue (Class|Enemy|GetIsDamaged _asenemy))
          (if (not _returnvalue)
            (Class|Enemy|SetIsDamaged _asenemy true)
            (Utilities|IsValid _asenemy
              (:Is%20Valid
                (Utilities|Array|Add (Variables|/Game/Blueprints/MyTPSCharacter/MyCharacter.MyCharacter_C|GetEnemiesHittenByMe (.AsMy%20Character (Utilities|Casting|CastToMyCharacter (Game|Player|GetPlayerPawn _asenemy)))) _asenemy)
                (Development|PrintString 0 "attac")
                (|SendDamage _asenemy)
                (return false)))))))))

(fn ReceivedNotifyEnd
  (params (MeshComp :type Skeletal%20Mesh%20Component%20Object%20Reference) (Animation :type Anim%20Sequence%20Base%20Object%20Reference))
  (bind _asmy_character (Utilities|Casting|CastToMyCharacter (Game|GetPlayerCharacter MeshComp)))
  (Utilities|FlowControl|Sequence
    (:then_0
      (if (not (Variables|/Game/Blueprints/MyTPSCharacter/MyCharacter.MyCharacter_C|GetisAttackAnimationPaused? _asmy_character))
        (Default|RemoveList(Buggysheet) _asmy_character)))
    (:then_1
      (Variables|/Game/Blueprints/MyTPSCharacter/MyCharacter.MyCharacter_C|SetCanAttackHitPause _asmy_character true)
      (return true))))