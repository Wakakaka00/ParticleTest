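; Third-person camera component for the player character that drives spring arm offset and length for default and boss combat views.
; SetCameraState starts a looping timer, set to one frame's delta, that runs the current mode instead of Tick.
; Combat uses a raised, pulled-back view while the boss is throned; otherwise yaw angles pick a shoulder side and target distance adjusts arm length.
; All moves lerp by delta time; default mode restores captured values.
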(event Custom|DelayWithGivenTimr
  (params (Bool%20To%20Delay :type Boolean%20%28by%20ref%29) (Timer :type Float%20%28single-precision%29) (Value%20To%20Set%20After%20Delay :type Boolean))
  (Utilities|FlowControl|Delay Timer)
  (Development|PrintString "Hello")
  (|SetBy-RefVar Bool%20To%20Delay Value%20To%20Set%20After%20Delay))

(event EventBeginPlay
  (bind _asmy_character (Utilities|Casting|CastToMyCharacter (Components|GetOwner)))
  (Variables|Player|SetPlayer _asmy_character))

(event EventTick
  (params (DeltaSeconds :type Float%20%28single-precision%29)))

(fn SetCameraComponents
  (params (Camera :type Camera%20Component%20Object%20Reference) (SpringArm :type Spring%20Arm%20Component%20Object%20Reference) (LeftCameraPos :type Child%20Actor%20Component%20Object%20Reference) (RightCameraPos :type Child%20Actor%20Component%20Object%20Reference) (DefaultCameraPos :type Child%20Actor%20Component%20Object%20Reference) (MiddleCameraPos :type Child%20Actor%20Component%20Object%20Reference) (LeftCameraPosCloser :type Child%20Actor%20Component%20Object%20Reference) (RightCameraPosCloser :type Child%20Actor%20Component%20Object%20Reference))
  (Variables|Default|SetCamera Camera)
  (Variables|Default|SetSpringArm SpringArm)
  (Variables|Default|SetLeft%20Camera%20Pos LeftCameraPos)
  (Variables|Default|SetRight%20Camera%20Pos RightCameraPos)
  (Variables|Default|SetDefault%20Camera%20Pos DefaultCameraPos)
  (Variables|Default|SetMiddle%20Camera%20Pos MiddleCameraPos)
  (Variables|Default|SetLeft%20Camera%20Pos%20Closer LeftCameraPosCloser)
  (Variables|Default|SetRight%20Camera%20Pos%20Closer RightCameraPosCloser)
  (Variables|Default|SetDefaultTargetCameraLength%28Ground%29 (Variables|/Script/Engine.SpringArmComponent|GetTargetArmLength (Variables|Default|GetSpringArm)))
  (Variables|Default|SetDefaultSocketOffset%28Ground%29 (Variables|/Script/Engine.SpringArmComponent|GetSocketOffset (Variables|Default|GetSpringArm)))
  (Variables|Default|SetDefaultSocketOffset%28Throne%29 (+ (Variables|/Script/Engine.SpringArmComponent|GetSocketOffset (Variables|Default|GetSpringArm)) "0, 0,200.000000"))
  (Variables|Default|SetDefaultTargetCameraLength%28Throne%29 (+ (Variables|/Script/Engine.SpringArmComponent|GetTargetArmLength (Variables|Default|GetSpringArm)) 4e+02)))

(fn CameraStateManagement
  (switch Utilities|FlowControl|Switch|SwitchonCamera_State_Enum (Variables|CameraState|GetCameraState)
    (:NewEnumerator0
      (|CombatMode))
    (:NewEnumerator2
      (|DefaultMode))))

(fn SetCameraState
  (params (State%20to%20Set :type Camera_State_Enum%20Enum :default "NewEnumerator0"))
  (Variables|CameraState|SetCameraState State%20to%20Set)
  (if (not (Utilities|Time|IsValidTimerHandle (Variables|Timers|GetCameraStateManagementTimerHandle)))
    (bind _returnvalue (Utilities|Time|SetTimerbyFunctionName self "CameraStateManagement" (Utilities|Time|GetWorldDeltaSeconds) true))
    (Variables|Timers|SetCameraStateManagementTimerHandle _returnvalue)))

(fn GetCameraState
  (return (Variables|CameraState|GetCameraState)))