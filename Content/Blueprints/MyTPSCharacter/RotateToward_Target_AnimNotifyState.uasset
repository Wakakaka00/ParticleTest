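; Anim notify state that turns MyCharacter during an animation, apparently for attacks, toward a close enemy or a cached attack direction.
; Each tick, unless the character is evading, it interpolates only the yaw along the shortest path toward TemperoryCloseEnemy.
; Without a valid enemy, it turns toward the non-zero CachedRotationBeforeAttack, used as a direction vector.
; Turn rate scales with Speed and frame time, with a fixed boost when tracking an enemy.
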(fn ReceivedNotifyTick
  (params (MeshComp :type Skeletal%20Mesh%20Component%20Object%20Reference) (Animation :type Anim%20Sequence%20Base%20Object%20Reference) (FrameDeltaTime :type Float%20%28single-precision%29))
  (bind _asmy_character (Utilities|Casting|CastToMyCharacter (Components|GetOwner MeshComp)))
  (if (not (Variables|/Game/Blueprints/MyTPSCharacter/MyCharacter.MyCharacter_C|GetisEvading _asmy_character))
    (Utilities|IsValid (Variables|/Game/Blueprints/MyTPSCharacter/MyCharacter.MyCharacter_C|GetTemperoryCloseEnemy _asmy_character)
      (:Is%20Valid
        (Transformation|SetActorRotation _asmy_character (Math|Rotator|Lerp(Rotator) (Math|Rotator|MakeRotator (.roll (Transformation|GetActorRotation _asmy_character)) (.pitch (Transformation|GetActorRotation _asmy_character)) (.yaw (Transformation|GetActorRotation _asmy_character))) (Math|Rotator|MakeRotator (.roll (Transformation|GetActorRotation _asmy_character)) (.pitch (Transformation|GetActorRotation _asmy_character)) (.yaw (Math|Rotator|FindLookatRotation (Transformation|GetActorLocation _asmy_character) (Transformation|GetActorLocation (Variables|/Game/Blueprints/MyTPSCharacter/MyCharacter.MyCharacter_C|GetTemperoryCloseEnemy _asmy_character))))) (* (+ (Variables|Default|GetSpeed) 2.0) FrameDeltaTime) true))
        (return false))
      (:Is%20Not%20Valid
        (if (> (Math|Vector|VectorLength (Variables|/Game/Blueprints/MyTPSCharacter/MyCharacter.MyCharacter_C|GetCachedRotationBeforeAttack _asmy_character)) 0.0)
          (Transformation|SetActorRotation _asmy_character (Math|Rotator|Lerp(Rotator) (Math|Rotator|MakeRotator (.roll (Transformation|GetActorRotation _asmy_character)) (.pitch (Transformation|GetActorRotation _asmy_character)) (.yaw (Transformation|GetActorRotation _asmy_character))) (Math|Rotator|MakeRotator (.roll (Transformation|GetActorRotation _asmy_character)) (.pitch (Transformation|GetActorRotation _asmy_character)) (.yaw (Math|Rotator|FindLookatRotation (Transformation|GetActorLocation _asmy_character) (+ (Transformation|GetActorLocation _asmy_character) (Variables|/Game/Blueprints/MyTPSCharacter/MyCharacter.MyCharacter_C|GetCachedRotationBeforeAttack _asmy_character))))) (* (Variables|Default|GetSpeed) FrameDeltaTime) true)))))))