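; Anim notify state that drives the evade movement of MyCharacter during an animation.
; On begin it caches the location of player pawn 0, rather than the mesh owner, in MoveTowardCashePlayerPositionBeforeMoving.
; Each tick it lerps the mesh owner horizontally along CachedRotationBeforeEvade, used as a direction vector, scaled by Units and Speed times delta time.
; The move is swept for collision, keeps the current Z and only runs when that cached vector is non-zero.
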(fn ReceivedNotifyTick
  (params (MeshComp :type Skeletal%20Mesh%20Component%20Object%20Reference) (Animation :type Anim%20Sequence%20Base%20Object%20Reference) (FrameDeltaTime :type Float%20%28single-precision%29))
  (bind _asmy_character (Utilities|Casting|CastToMyCharacter (Components|GetOwner MeshComp)))
  (if (> (Math|Vector|VectorLength (Variables|/Game/Blueprints/MyTPSCharacter/MyCharacter.MyCharacter_C|GetCachedRotationBeforeEvade _asmy_character)) 0.0)
    (Transformation|SetActorLocation _asmy_character (Math|Vector|Lerp(Vector) (Math|Vector|MakeVector (.x (Transformation|GetActorLocation _asmy_character)) (.y (Transformation|GetActorLocation _asmy_character)) (.z (Transformation|GetActorLocation _asmy_character))) (Math|Vector|MakeVector (.x (+ (* (Variables|/Game/Blueprints/MyTPSCharacter/MyCharacter.MyCharacter_C|GetCachedRotationBeforeEvade _asmy_character) (Variables|Default|GetUnits)) (Transformation|GetActorLocation _asmy_character))) (.y (+ (* (Variables|/Game/Blueprints/MyTPSCharacter/MyCharacter.MyCharacter_C|GetCachedRotationBeforeEvade _asmy_character) (Variables|Default|GetUnits)) (Transformation|GetActorLocation _asmy_character))) (.z (Transformation|GetActorLocation _asmy_character))) (* (Variables|Default|GetSpeed) FrameDeltaTime)) true false)
    (return false)))

(fn ReceivedNotifyBegin
  (params (MeshComp :type Skeletal%20Mesh%20Component%20Object%20Reference) (Animation :type Anim%20Sequence%20Base%20Object%20Reference) (TotalDuration :type Float%20%28single-precision%29))
  (bind _asmy_character (Utilities|Casting|CastToMyCharacter (Game|Player|GetPlayerPawn MeshComp)))
  (Variables|/Game/Blueprints/MyTPSCharacter/MyCharacter.MyCharacter_C|SetMoveToward-CashePlayerPositionBeforeMoving _asmy_character (Transformation|GetActorLocation _asmy_character))
  (return false))