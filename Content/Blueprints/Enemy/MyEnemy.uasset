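; MyEnemy is an enemy Blueprint that can be targeted by a lock-on system.
; LockOnFlip toggles the LockOnSphere marker, and a look-at function rotates Sphere toward the player character.
; DistanceToPlayer line-traces to the player pawn, ignoring "Enemy"-tagged actors, stores the distance and sets CanBeTargeted unconditionally.
; DistanceToEnemies draws a debug trace toward a tagged enemy but returns inside its loop and stores no result.
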(event Custom|LockOnFlip
  (Utilities|FlowControl|FlipFlop
    (:A
      (Rendering|SetVisibility (Variables|Default|GetLockOnSphere) true false))
    (:B
      (Rendering|SetVisibility (Variables|Default|GetLockOnSphere) false false))))

(event EventBeginPlay)

(event Collision|EventActorBeginOverlap
  (params (OtherActor :type Actor%20Object%20Reference)))

(event EventTick
  (params (DeltaSeconds :type Float%20%28single-precision%29)))

(fn ConstructionScript
  (Variables|Default|SetsphereLooker (Variables|Default|GetSphere)))

(fn DistancetoPlayer
  (bind _outactors (Actor|GetAllActorswithTag "Enemy"))
  (bind _outhit (Collision|LineTraceForObjects (Transformation|GetActorLocation) (Transformation|GetActorLocation (Game|Player|GetPlayerPawn 0)) (Utilities|Array|MakeArray "ObjectTypeQuery3") false _outactors "ForDuration" true "(R=1.000000,G=0.000000,B=0.000000,A=1.000000)" "(R=0.000000,G=1.000000,B=0.000000,A=1.000000)" 0.1))
  (Variables|Default|SetPlayerToEnemyDistance (.Distance (Collision|BreakHitResult _outhit)))
  (Variables|Default|SetCanBeTargeted true)
  (return))

(fn DistancetoEnemies
  (bind _outactors (Actor|GetAllActorswithTag "Enemy"))
  (for _array_element _outactors
    (bind _asmy_enemy (Utilities|Casting|CastToMyEnemy _array_element))
    (Collision|LineTraceForObjects (Transformation|GetActorLocation) (Transformation|GetActorLocation _asmy_enemy) (Utilities|Array|MakeArray "ObjectTypeQuery2") false (Utilities|Array|MakeArray self) "ForDuration" true "(R=0.000000,G=1.000000,B=0.105227,A=1.000000)" "(R=0.000000,G=1.000000,B=0.000000,A=1.000000)" 0.1)
    (return)))

(fn SphereLookat
  (Transformation|SetWorldRotation (Variables|Default|GetSphere) (Math|Rotator|FindLookatRotation (Transformation|GetWorldLocation (Variables|Default|GetSphere)) (Transformation|GetActorLocation (Game|GetPlayerCharacter 0))) false false))