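; Minion grenade actor that explodes after a timed fuse, damaging and pushing back player characters caught in the blast.
; The explosion collision stays disabled from BeginPlay until Explode enables it, spawns the explosion particle and destroys the actor at once.
; Overlaps with Player-tagged components call PushBack with the normalized player-to-grenade vector, then apply custom damage through MyCharacter.
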(event OnComponentBeginOverlap(ExplosionCollision)
  (params (OverlappedComponent :type Primitive%20Component%20Object%20Reference) (OtherActor :type Actor%20Object%20Reference) (OtherComp :type Primitive%20Component%20Object%20Reference) (OtherBodyIndex :type Integer) (bFromSweep :type Boolean) (SweepResult :type Hit%20Result%20Structure%20%28by%20ref%29))
  (bind _returnvalue (Components|GetOwner OtherComp))
  (if (Components|ComponentHasTag OtherComp "Player")
    (bind _astpscharacter (Utilities|Casting|CastToTPSCharacter _returnvalue))
    (Class|TPSCharacter|PushBack _astpscharacter 1.5e+03 (Math|Vector|Normalize (- (Transformation|GetWorldLocation (Variables|Default|GetSphere)) (Transformation|GetActorLocation _returnvalue))))
    (bind _asmy_character (Utilities|Casting|CastToMyCharacter _returnvalue))
    (Default|ApplyCustomDamage _asmy_character 15.0 "NewEnumerator0" 0.0 0.0)))

(event Custom|Explode
  (Collision|SetCollisionEnabled (Variables|Default|GetExplosionCollision) "QueryAndPhysics")
  (Effects|SpawnEmitteratLocation "/Game/Explosions/Particles/P_Explosive1.P_Explosive1" (Transformation|GetWorldLocation (Variables|Default|GetSphere)))
  (Actor|DestroyActor))

(event EventBeginPlay
  (Collision|SetCollisionEnabled (Variables|Default|GetExplosionCollision) "NoCollision")
  (Utilities|FlowControl|Delay (Variables|Default|GetexplodeDuration))
  (CallFunction|Explode))

(fn ConstructionScript)