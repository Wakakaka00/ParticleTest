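; Boss blood pool actor that spawns minions above itself and registers each one with the boss's AI controller.
; Start pools spawn one minion immediately and destroy themselves after a short delay.
; Other pools add themselves to the boss's BloodPoolList for a limited lifetime, then remove themselves and are destroyed.
; While alive, those pools use Tick to spawn minions at randomized intervals whenever the controller's minion list is below its cap.
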(event Custom|RandomizeDuration
  (Variables|Default|SetspawnDuration (Math|Random|RandomFloatinRange 5.0 1e+01)))

(event Custom|SpawnEnemy
  (bind _returnvalue (Game|SpawnActorfromClass "/Game/Minion/Minion_BP.Minion_BP_C" (Math|Conversions|ToTransform(Vector) (+ (Transformation|GetActorLocation) "0, 0,100.000000")) "AdjustIfPossibleButAlwaysSpawn" 0 0))
  (bind _asmy_aicontroller (Utilities|Casting|CastToMyAIController (AI|GetAIController (Variables|Default|GetBossActor))))
  (Class|MyAIController|AddMinion _asmy_aicontroller _returnvalue))

(event EventBeginPlay
  (bind _self self)
  (bind _outactors (Actor|GetAllActorsOfClass "/Game/Boss/MyBossCharacter.MyBossCharacter_C"))
  (Variables|Default|SetBossActor (Utilities|Array|Get(acopy) _outactors))
  (if (Variables|Default|GetisStart)
    (CallFunction|SpawnEnemy)
    (Utilities|FlowControl|Delay 1e+01)
    (Actor|DestroyActor)
    (else
      (CallFunction|RandomizeDuration)
      (bind _outactors_2 (Actor|GetAllActorsOfClass "/Game/Boss/MyBossCharacter.MyBossCharacter_C"))
      (bind _output_get (Variables|Default|SetBossActor (Utilities|Array|Get(acopy) _outactors_2)))
      (bind _asboss_character (Utilities|Casting|CastToBossCharacter _output_get))
      (Utilities|Array|Add (Variables|/Script/ParticleTest.BossCharacter|GetbloodPoolList _asboss_character) _self)
      (Utilities|FlowControl|Delay 2e+01)
      (Utilities|Array|RemoveItem (Variables|/Script/ParticleTest.BossCharacter|GetbloodPoolList _asboss_character) _self)
      (Actor|DestroyActor))))

(event EventTick
  (params (DeltaSeconds :type Float%20%28single-precision%29))
  (bind _asmy_aicontroller (Utilities|Casting|CastToMyAIController (AI|GetAIController (Variables|Default|GetBossActor))))
  (if (< (Utilities|Array|Length (Variables|/Script/ParticleTest.MyAIController|GetMinionList _asmy_aicontroller)) 5)
    (if (not (Variables|Default|GetisStart))
      (bind _output_get (Variables|Default|SetspawnTimer (+ (Variables|Default|GetspawnTimer) DeltaSeconds)))
      (if (>= _output_get (Variables|Default|GetspawnDuration))
        (CallFunction|SpawnEnemy)
        (Variables|Default|SetspawnTimer 0.0)
        (CallFunction|RandomizeDuration)))))

(fn ConstructionScript)