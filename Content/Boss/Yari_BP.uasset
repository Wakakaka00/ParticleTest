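; Boss spear (yari) projectile that can be thrown at the player from the boss's throne attack and deal damage.
; The throw event enables trigger collisions and physics, detaches the spear, aims it at the player with a pitch offset, and launches it with a scaled suggested-projectile-velocity impulse using the boss's launch speed.
; A separate damage event applies fixed custom damage to the player character, with no caller in this graph.
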(event EventDamagePlayer
  (bind _asmy_character (Utilities|Casting|CastToMyCharacter (Game|GetPlayerCharacter 0)))
  (Default|ApplyCustomDamage _asmy_character 2e+01 "NewEnumerator0" 0.0 0.0))

(event EventThrowonThrone
  (bind _returnvalue (Transformation|GetActorLocation))
  (bind _returnvalue_2 (Game|GetPlayerCharacter 0))
  (bind _returnvalue_3 (Transformation|GetActorLocation _returnvalue_2))
  (bind _returnvalue_4 (Math|Rotator|FindLookatRotation _returnvalue _returnvalue_3))
  (Collision|SetCollisionProfileName (Variables|Default|GetTriggerBox) "Trigger" :!class /Script/Engine.PrimitiveComponent)
  (Collision|SetCollisionProfileName (Variables|Default|GetTriggerCapsule) "Trigger" :!class /Script/Engine.PrimitiveComponent)
  (Physics|SetSimulatePhysics (Variables|Default|GetStaticMeshComponent) true)
  (Variables|Default|SetisThrowing true)
  (Transformation|DetachFromActor "KeepWorld" "KeepWorld" "KeepWorld")
  (bind _tossvelocity (Class|GameplayStatics|BlueprintSuggestProjectileVelocity _returnvalue _returnvalue_3 (Variables|/Script/ParticleTest.BossCharacter|GetyariLaunchSpeed (Variables|Default|GetbossActor)) 0.0 "DoNotTrace" 0.0 false false))
  (Transformation|SetActorRotation (Math|Rotator|MakeRotator (.roll _returnvalue_4) (- (.pitch _returnvalue_4) 9e+01) (.yaw _returnvalue_4)))
  (Physics|AddImpulse (Variables|Default|GetStaticMeshComponent) (* _tossvelocity 1.5) "None" false))

(fn ConstructionScript)