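; Torii gate actor that starts the boss encounter when the player enters the arena.
; On overlap by a component tagged Player, it reaches the boss's AI controller through the player character's BossActor reference and sets IsEnterArena.
; It then disables the trigger collision and enables the Wall's collision.
; A delayed ThrowYari call on the controller is left unconnected.
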(event OnComponentBeginOverlap(Trigger)
  (params (OverlappedComponent :type Primitive%20Component%20Object%20Reference) (OtherActor :type Actor%20Object%20Reference) (OtherComp :type Primitive%20Component%20Object%20Reference) (OtherBodyIndex :type Integer) (bFromSweep :type Boolean) (SweepResult :type Hit%20Result%20Structure%20%28by%20ref%29))
  (if (Components|ComponentHasTag OtherComp "Player")
    (bind _astpscharacter (Utilities|Casting|CastToTPSCharacter (Game|GetPlayerCharacter 0)))
    (bind _asmy_aicontroller (Utilities|Casting|CastToMyAIController (Pawn|GetController (Variables|/Script/ParticleTest.TPSCharacter|GetbossActor _astpscharacter))))
    (Variables|/Script/ParticleTest.MyAIController|SetisEnterArena _asmy_aicontroller true)
    (Collision|SetCollisionEnabled (Variables|Default|GetTrigger) "NoCollision")
    (Collision|SetCollisionEnabled (Variables|Default|GetWall) "QueryAndPhysics")))

(fn ConstructionScript)